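; BP_Security_Guard is an enemy guard that patrols and chases the player when spotted.
; PawnSensing starts an AI MoveTo chase and uses a retriggerable delay to resume patrolling when sightings stop.
; Tick sends it back to spawn beyond a leash distance, otherwise issues delayed random nearby patrol moves while the player is unseen.
; The catch overlap only casts to the player, and a chase range check is disconnected.
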(event OnComponentBeginOverlap(CollisionMesh)
  (params (OverlappedComponent :type Primitive%20Component%20Object%20Reference) (OtherActor :type Actor%20Object%20Reference) (OtherComp :type Primitive%20Component%20Object%20Reference) (OtherBodyIndex :type Integer) (bFromSweep :type Boolean) (SweepResult :type Hit%20Result%20Structure%20%28by%20ref%29))
  ;[1 1 1] getting caught
  (Utilities|Casting|CastToBP_ThirdPersonCharacter OtherActor))

(event OnSeePawn(PawnSensing)
  (params (Pawn :type Pawn%20Object%20Reference))
  ;[1 1 1] pawn sensing
  (bind _asbp_third_person_character (Utilities|Casting|CastToBP_ThirdPersonCharacter Pawn))
  (Utilities|FlowControl|Sequence
    (:then_0
      (Variables|Default|SetCanSeePlayer true)
      (CallFunction|ChasePlayer))
    (:then_1
      (Utilities|FlowControl|RetriggerableDelay 1.0)
      (Variables|Default|SetCanSeePlayer false)
      (CallFunction|Patrol))))

(event Custom|ChasePlayer
  ;[1 1 1] chase player
  (AI|AIMoveTo self "0, 0, 0" (Game|GetPlayerCharacter 0) 7.0 false))

(event Custom|Patrol
  ;[1 1 1] patrol
  (AI|AIMoveTo self (.RandomLocation (AI|Navigation|GetRandomReachablePointinRadius (Transformation|GetActorLocation) 5e+02 0 0)) 0 5.0 false))

(event EventBeginPlay
  (Variables|Default|SetSpawnLocation (Transformation|GetActorLocation)))

(event EventTick
  (params (DeltaSeconds :type Float%20%28single-precision%29))
  (bind _spawnlocation (Variables|Default|GetSpawnLocation))
  ;[1 1 1] go back to spawn location
  (if (> (Math|Vector|Distance(Vector) (Transformation|GetActorLocation) _spawnlocation) 2e+03)
    (AI|AIMoveTo 0 _spawnlocation 0 5.0 false)
    (elif (not (Variables|Default|GetCanSeePlayer))
      (Utilities|FlowControl|Delay 3.0)
      (CallFunction|Patrol))))

(fn ConstructionScript)